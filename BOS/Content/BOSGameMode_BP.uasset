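; BOSGameMode_BP is a game mode that tracks lives for two teams of BOSBall_BP balls and respawns dead ones.
; BeginPlay copies both team life counts into BOSGameState.
; Every Tick it polls all balls, decrements the life count for each dead ball's PlayerState team, and updates the GameState.
; It then destroys that ball and tells its BallController to respawn, without checking remaining lives.
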(event EventBeginPlay
  (bind _asbosgame_state (Utilities|Casting|CastToBOSGameState (Game|GetGameState)))
  (Variables|/Script/BOS.BOSGameState|SetTeamALives _asbosgame_state (Variables|Default|GetNumTeamA))
  (Variables|/Script/BOS.BOSGameState|SetTeamBLives _asbosgame_state (Variables|Default|GetNumTeamB)))

(event EventTick
  (params (DeltaSeconds :type Float%20%28single-precision%29))
  (bind _outactors (Actor|GetAllActorsOfClass "/Game/BOSBall_BP.BOSBall_BP_C"))
  (for _array_element _outactors
    (if (Variables|/Script/BOS.BOSBall|GetbIsDead _array_element)
      (bind _asbosplayer_state (Utilities|Casting|CastToBOSPlayerState (Variables|/Script/Engine.Pawn|GetPlayerState _array_element)))
      (if (Variables|/Script/BOS.BOSPlayerState|GetbTeamB _asbosplayer_state)
        (bind _output_get (Variables|Default|SetNumTeamB (- (Variables|Default|GetNumTeamB) 1)))
        (else
          (bind _output_get_2 (Variables|Default|SetNumTeamA (- (Variables|Default|GetNumTeamA) 1)))))
      (bind _asbosgame_state (Utilities|Casting|CastToBOSGameState (Game|GetGameState)))
      (Variables|/Script/BOS.BOSGameState|SetTeamALives _asbosgame_state _output_get_2)
      (Variables|/Script/BOS.BOSGameState|SetTeamBLives _asbosgame_state _output_get)
      (bind _asball_controller (Utilities|Casting|CastToBallController (Pawn|GetController _array_element)))
      (Actor|DestroyActor _array_element)
      (Class|BallController|Respawn _asball_controller))))

(fn ConstructionScript)